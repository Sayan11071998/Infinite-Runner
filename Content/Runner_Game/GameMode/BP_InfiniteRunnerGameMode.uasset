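; Infinite runner game mode that builds the starting track and runs the score counter.
; On BeginPlay a 20-pass loop calls AddMap, which spawns a BP_LevelFloor at NextSpawnPoint and takes that floor's attach transform as the next spawn point, chaining segments.
; The same loop body also adds a WBP_UI_HUD to the viewport and sets the looping timer whose IncrementScore call raises ScoreCount.
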(event EventBeginPlay
  ;[1 1 1] Procedural Level Generation
  (for _index (range 0 19)
    (CallFunction|AddMap)
    ;[1 1 1] Create UI and Display
    (bind _returnvalue (UserInterface|CreateWidget "/Game/Runner_Game/UI/WBP_UI_HUD.WBP_UI_HUD_C"))
    (UserInterface|Viewport|AddtoViewport _returnvalue 0)
    (bind _returnvalue_2 (Utilities|Time|SetTimerbyFunctionName 0 "IncrementScore" 0.6 true))
    (Variables|Default|SetTimerHandler _returnvalue_2)))

(fn ConstructionScript)

(fn AddMap
  (bind _returnvalue (Game|SpawnActorfromClass "/Game/Runner_Game/Gameplay_Items/BP_LevelFloor.BP_LevelFloor_C" (Variables|Default|GetNextSpawnPoint) "Undefined" 0 0))
  (bind _output_get (Variables|Default|SetLevelREF _returnvalue))
  (bind _attachpoint (Default|GetAttachTransform _output_get))
  (Variables|Default|SetNextSpawnPoint _attachpoint))

(fn IncrementScore
  (bind _result (Math|Integer|IncrementInt (Variables|Default|GetScoreCount))
    (:%20%20
      (Variables|Default|SetScoreCount _result))))